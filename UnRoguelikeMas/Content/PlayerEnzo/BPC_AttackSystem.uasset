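; Player attack component for BP_PlayerEnzo that plays melee combo montages for one-handed, two-handed and spear weapons.
; Attack input, gated by PuedeAtacar, starts a montage picked by the owner's weapon flags and combo index, or queues a follow-up if already attacking.
; The Nose event consumes the queued hit or resets the combo.
; On continuation, its Sequence fires the weapon check plus both two-handed and spear montages unconditionally.
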(event `self.ReceiveBeginPlay`
  (bind _asbp_player_enzo_ (cast `/Game/PlayerEnzo/BP_PlayerEnzo+` (`self.GetOwner`)))
  (bind _output_get (set `self.As BP Player Enzo+` _asbp_player_enzo_))
  (set `self.CharacterMesh` (`Character.Mesh` _output_get))
  (bind (_stats_cost _stats_mesh _stats_damage _stats_socket _stats_tipodearma _stats_tipode2manos) (break `/Game/Weapons/S_WeaponStats` (`/Game/PlayerEnzo/BP_PlayerEnzo+.Stats` _output_get)))
  (set `self.tipoDeArma` _stats_tipodearma)
  (set `self.tipoDeArma2` _stats_tipode2manos))

(event `Stop Combo`
  ; Detener combo de ataque
  (set `self.estaAtacando?` false)
  (set `self.indiceDeAtaque` 0))

(event `EnhancedInput|/Game/PlayerEnzo/Input/Actions/IA_Attack`
  (params (ActionValue :type Boolean) (ElapsedSeconds :type "Float (double-precision)") (TriggeredSeconds :type "Float (double-precision)") (InputAction :type "InputAction Object Reference" :default "/Game/PlayerEnzo/Input/Actions/IA_Attack.IA_Attack"))
  ; Input de ataque
  (:`Started`
    (if (`self.puedeAtacar?`)
      (`self.Attack`))))

(event `Attack`
  (bind _as_bp_player_enzo_ (`self.As BP Player Enzo+`))
  ; Logica de animaciones de ataque
  (if (`self.estaAtacando?`)
    (set `self.ataco` true)
    (else
      (set `self.estaAtacando?` true)
      (if (`/Game/PlayerEnzo/BP_PlayerEnzo+.1MWeapon` _as_bp_player_enzo_) :!label _label
        (`|PlayMontage` (`self.CharacterMesh`) (`self.1HandWeapon`)
          (:`then`
            (`/Engine/EditorBlueprintResources/StandardMacros.IncrementInt` (`self.indiceDeAtaque`))))
        (elif (not (`/Game/PlayerEnzo/BP_PlayerEnzo+.TipoLanza` _as_bp_player_enzo_))
          (`|PlayMontage` (`self.CharacterMesh`) (`self.2HandWeapon`) :!label _label_2
            (:`then`
              (`/Engine/EditorBlueprintResources/StandardMacros.IncrementInt` (`self.indiceDeAtaque`))))
          (else
            (`|PlayMontage` (`self.CharacterMesh`) (`self.Lanza`) :!label _label_3
              (:`then`
                (`/Engine/EditorBlueprintResources/StandardMacros.IncrementInt` (`self.indiceDeAtaque`))))))))))

(event `Nose`
  ; Continuar combo de ataque
  (if (`self.ataco`)
    (set `self.ataco` false)
    (`|ExecutionSequence`
      (:`then_0`
        (goto _label))
      (:`then_1`
        (goto _label_2))
      (:`then_2`
        (goto _label_3)))
    (else
      (`self.Stop Combo`))))

(fn `1HandWeapon`
  (returns (`Anim montage` :type "AnimMontage Object Reference"))
  (return (select `int` (`self.indiceDeAtaque`) :`0` "/Game/PlayerEnzo/Animaciones/AnimacionesPlayerEnzo/1Mano/AnimacionDeAtaque/Montages_Finales/AM_Ataque1.AM_Ataque1" :`1` "/Game/PlayerEnzo/Animaciones/AnimacionesPlayerEnzo/1Mano/AnimacionDeAtaque/Montages_Finales/AM_Ataque2.AM_Ataque2" :`2` null :!type "AnimMontage Object Reference")))

(fn `2HandWeapon`
  (returns (`Anim montage` :type "AnimMontage Object Reference"))
  (return (select `int` (`self.indiceDeAtaque`) :`0` "/Game/PlayerEnzo/Animaciones/AnimacionesPlayerEnzo/2Manos/AM_Ataque2mano2.AM_Ataque2mano2" :`1` "/Game/PlayerEnzo/Animaciones/AnimacionesPlayerEnzo/2Manos/AM_Ataque2manos.AM_Ataque2manos" :`2` null :!type "AnimMontage Object Reference")))

(fn `Lanza`
  (returns (`Anim montage` :type "AnimMontage Object Reference"))
  (return (select `int` (`self.indiceDeAtaque`) :`0` "/Game/PlayerEnzo/Animaciones/AnimacionesPlayerEnzo/2Manos/AtaquesLanza/AM_AtaqueLanza1.AM_AtaqueLanza1" :`1` "/Game/PlayerEnzo/Animaciones/AnimacionesPlayerEnzo/2Manos/AtaquesLanza/AM_ataqueLanza3.AM_ataqueLanza3" :`2` "/Game/PlayerEnzo/Animaciones/AnimacionesPlayerEnzo/2Manos/AtaquesLanza/AM_ataqueLanza3.AM_ataqueLanza3" :!type "AnimMontage Object Reference")))