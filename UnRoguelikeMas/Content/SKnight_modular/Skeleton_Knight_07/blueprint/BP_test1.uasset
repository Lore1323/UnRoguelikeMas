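; BP_test1 is a test Blueprint for the modular Skeleton Knight 07, assembled from several skeletal mesh components.
; Its Construction Script calls SetLeaderPoseComponent on the part components so that they follow the pose of Mesh and animate as one body.
; SkeletalMesh7 is wired into that call twice, and the file shows no other logic.
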(fn `UserConstructionScript`
  (`SkinnedMeshComponent.SetLeaderPoseComponent` (`self.SkeletalMesh7`) (`self.Mesh`) false false)
  (`SkinnedMeshComponent.SetLeaderPoseComponent` (`self.SkeletalMesh2`) (`self.Mesh`) false false)
  (`SkinnedMeshComponent.SetLeaderPoseComponent` (`self.SkeletalMesh3`) (`self.Mesh`) false false)
  (`SkinnedMeshComponent.SetLeaderPoseComponent` (`self.SkeletalMesh4`) (`self.Mesh`) false false)
  (`SkinnedMeshComponent.SetLeaderPoseComponent` (`self.SkeletalMesh5`) (`self.Mesh`) false false)
  (`SkinnedMeshComponent.SetLeaderPoseComponent` (`self.SkeletalMesh6`) (`self.Mesh`) false false)
  (`SkinnedMeshComponent.SetLeaderPoseComponent` (`self.SkeletalMesh7`) (`self.Mesh`) false false)
  (`SkinnedMeshComponent.SetLeaderPoseComponent` (`self.SkeletalMesh`) (`self.Mesh`) false false)
  (`SkinnedMeshComponent.SetLeaderPoseComponent` (`self.SkeletalMesh1`) (`self.Mesh`) false false)
  (`SkinnedMeshComponent.SetLeaderPoseComponent` (`self.SkeletalMesh8`) (`self.Mesh`) false false))