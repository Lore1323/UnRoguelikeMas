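; BP_MyGameInstance is a game instance that tracks cleared rooms and derives the difficulty level from that count, within the wave system folder.
; AvisarSalaDespejada increments SalasDespejadas, then raises NivelDeDificultad to 2 and later to 3 as the count reaches two thresholds.
; ObtenerDificultadActual returns the current level to callers.
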(event `/Game/MapaProcedural/BPI_GestorDeDificultad.AvisarSalaDespejada`
  (bind _result (`/Engine/EditorBlueprintResources/StandardMacros.IncrementInt` (`self.salasDespejadas`))
    (:`  `
      (if (>= _result 4)
        (set `self.nivelDeDificultad` 2)
        (if (>= (`self.salasDespejadas`) 10)
          (set `self.nivelDeDificultad` 3))))))

(fn `ObtenerDificultadActual`
  (returns (dificultad :type Integer))
  (return (`self.nivelDeDificultad`)))