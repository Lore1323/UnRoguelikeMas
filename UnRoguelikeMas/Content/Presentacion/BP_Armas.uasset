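; BP_Armas is a weapon pickup actor that gives the player a weapon chosen by its Index.
; At construction it looks up the matching DT_Weapons row by that index, stores it as Stats and applies its skeletal mesh, so the editor previews the weapon.
; When BP_PlayerEnzo overlaps the box, it sets the player's WeaponIndex and calls SetStats to update the player's weapon data.
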(event `self.Box.OnComponentBeginOverlap`
  (params (OverlappedComponent :type "PrimitiveComponent Object Reference") (OtherActor :type "Actor Object Reference") (OtherComp :type "PrimitiveComponent Object Reference") (OtherBodyIndex :type Integer) (bFromSweep :type Boolean) (SweepResult :type "HitResult Structure (by ref)"))
  (bind _asbp_player_enzo_ (cast `/Game/PlayerEnzo/BP_PlayerEnzo+` OtherActor))
  (set `/Game/PlayerEnzo/BP_PlayerEnzo+.WeaponIndex` (`self.Index`) _asbp_player_enzo_)
  (`/Game/PlayerEnzo/BP_PlayerEnzo+.SetStats` _asbp_player_enzo_))

(fn `SetMesh`
  (bind (_stats_cost _stats_mesh) (break `/Game/Weapons/S_WeaponStats` (`self.Stats`)))
  (bind _returnvalue (`|GetDataTableRow` "/Game/Weapons/DT_Weapons.DT_Weapons" (`KismetStringLibrary.Conv_StringToName` (`KismetStringLibrary.Conv_IntToString` (`self.Index`))))
    (:`then`
      (set `self.Stats` _returnvalue)
      (`SkeletalMeshComponent.SetSkeletalMeshAsset` (`self.SkeletalMesh`) _stats_mesh))))

(fn `UserConstructionScript`
  (`self.SetMesh`))