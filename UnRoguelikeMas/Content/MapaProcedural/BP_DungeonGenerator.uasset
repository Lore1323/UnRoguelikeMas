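; Procedural dungeon generator actor that spawns a start room on BeginPlay, then chains random rooms until a room counter runs out.
; Each room spawns at a random open exit; after a short delay, overlapping rooms are destroyed and retried, while valid ones add their exits to the pool.
; On completion it caps unused exits with doors.
; A looping watchdog timer opens Lvl_ThirdPerson if generation is still running at 120 seconds of game time.
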(event `SpawnStartRoom`
  ;[0.0421 0.15 0.000244 0.5] Spawn Start Room
  (bind _returnvalue (`|SpawnActorFromClass` "/Game/Medieval_Sewer_Dungeon/Blueprints/Empty_Tunnel/SalasAUsar/BP_Room3.BP_Room3_C" (`SceneComponent.GetRelativeTransform` (`self.DefaultSceneRoot`)) "AlwaysSpawn" "MultiplyWithRoot" null null))
  (`KismetArrayLibrary.Array_Append` (`self.ExitList`) (`SceneComponent.GetChildrenComponents` (`/Game/Medieval_Sewer_Dungeon/Blueprints/Tunnel_Master.ExitsFolder` _returnvalue) true))
  (`KismetSystemLibrary.PrintString` "1"))

(event `SpawnNextRoom`
  ;[0.004538 0.04602 0.15 0.5] ConectarSiguienteSala
  (bind _output_get (set `self.SelectedExitPoint` (`KismetArrayLibrary.Array_Random` (`self.ExitList`))))
  (bind _returnvalue (`|SpawnActorFromClass` (`KismetArrayLibrary.Array_Random` (`self.RoomList`)) (`SceneComponent.K2_GetComponentToWorld` _output_get) "AlwaysSpawn" "MultiplyWithRoot" null null))
  (bind _astunnel_master (cast `/Game/Medieval_Sewer_Dungeon/Blueprints/Tunnel_Master` _returnvalue)
    (:`then`
      (set `self.LastDoor` _astunnel_master)
      (`KismetSystemLibrary.Delay` 0.2)
      (`self.CheckForOverlap`))
    (:`CastFailed`
      (`KismetSystemLibrary.PrintString` "Cast Failed"))))

(event `Add OverlappedList`
  ;[0.15 0.003725 0 0.5] Crea lista si hay actores overlapeados
  (for _array_element (`SceneComponent.GetChildrenComponents` (`/Game/Medieval_Sewer_Dungeon/Blueprints/Tunnel_Master.OverlapedFolder` (`self.LastDoor`)) false)
    (bind _asbox_collision (cast `BoxComponent` _array_element))
    (`KismetArrayLibrary.Array_Append` (`self.OverlappedList`) (`PrimitiveComponent.GetOverlappingComponents` _asbox_collision))))

(event `CheckForOverlap`
  ;[0.06294 0.01557 0.15 0.5] Revisar que las salas no colisionen entre si
  (`self.Add OverlappedList`)
  (if (`KismetArrayLibrary.Array_IsNotEmpty` (`self.OverlappedList`))
    (`KismetArrayLibrary.Array_Clear` (`self.OverlappedList`))
    (`self.K2_DestroyActor` (`self.LastDoor`))
    (`self.SpawnNextRoom`)
    (else
      (set `self.CantidadDeSalas` (- (`self.CantidadDeSalas`) 1))
      (`KismetArrayLibrary.Array_RemoveItem` (`self.ExitList`) (`self.SelectedExitPoint`))
      (`KismetArrayLibrary.Array_Append` (`self.ExitList`) (`SceneComponent.GetChildrenComponents` (`/Game/Medieval_Sewer_Dungeon/Blueprints/Tunnel_Master.ExitsFolder` (`self.LastDoor`)) true))
      (if (> (`self.CantidadDeSalas`) 0)
        (`self.SpawnNextRoom`)
        (else
          (`KismetSystemLibrary.Delay` 1.0)
          (`self.ClosingOpenDoors`)
          (set `self.DungeonComplete` true)
          (`KismetSystemLibrary.K2_ClearAndInvalidateTimerHandle` (`self.Timer Handle`))
          (`KismetSystemLibrary.PrintString` "DUNGEON COMPLETE" true true (struct :`R` 0.697917 :`G` 0.16701 :`A` 1.0)))))))

(event `ClosingOpenDoors`
  (for _array_element (`self.ExitList`)
    (`|SpawnActorFromClass` "/Game/Medieval_Sewer_Dungeon/Blueprints/Props/BP_Door.BP_Door_C" (`SceneComponent.K2_GetComponentToWorld` _array_element) "AlwaysSpawn" "MultiplyWithRoot" null null)))

(event `self.ReceiveBeginPlay`
  (`self.SpawnStartRoom`)
  (`self.StartDungeonTimer`)
  (`self.SpawnNextRoom`))

(event `StartDungeonTimer`
  (bind _returnvalue (`KismetSystemLibrary.K2_SetTimerDelegate` (delegate `CheckForDungeonComplete`) 1.0 true))
  (set `self.Timer Handle` _returnvalue))

(event `CheckForDungeonComplete`
  (`KismetSystemLibrary.PrintString` "Running Timer")
  (if (>= (`KismetSystemLibrary.GetGameTimeInSeconds`) 120.0)
    (`GameplayStatics.OpenLevel` "Lvl_ThirdPerson")))

(fn `UserConstructionScript`)