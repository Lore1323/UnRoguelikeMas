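; BP_Doors is an interactable sliding door for the procedural map, configured from the "Door" row of the interactable list data table.
; A timeline lerps the root component from its starting location by the PosFinal offset, with sweep.
; The first interaction plays the timeline through a DoOnce that is never reset.
; DesbloquearPuerta and BloquearPuerta set EstaBloqueada and play or reverse the timeline, but interaction never checks that flag.
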(event `self.ReceiveBeginPlay`
  (`InteractableComponent.SetInteractableDataBasedOnDataTable` (`self.Interactable`) "/CustomizableInteractionPlugin/Blueprint/Interactables/DT_CIP_InteractableList.DT_CIP_InteractableList" "Door")
  (set `self.posInicial` (`SceneComponent.K2_GetComponentToWorld` (`self.Door`))))

(event `self.Interactable.OnOverlapUpdated`
  (params (bIsOverlapping :type Boolean) (OverlappingInteractor :type "InteractorComponent Object Reference") (Interactable :type "InteractableComponent Object Reference"))
  (bind _returnvalue (`GameplayStatics.GetActorOfClass` "/Game/PlayerEnzo/BP_PlayerEnzo+.BP_PlayerEnzo+_C"))
  (set `self.player` _returnvalue))

(event `DesbloquearPuerta`
  (bind _posinicial_location (`KismetMathLibrary.BreakTransform` (`self.posInicial`)))
  (bind _posfinal_location (`KismetMathLibrary.BreakTransform` (`self.posFinal`)))
  (set `self.estaBloqueada?` false)
  (bind (_direction _alpha) (`Timeline|TL_OpenDoor` :!label _label)
    (:`Update`
      (`SceneComponent.K2_SetRelativeLocation` (`self.DefaultSceneRoot`) (`KismetMathLibrary.VLerp` _posinicial_location (+ _posinicial_location _posfinal_location) _alpha) true false))))

(event `self.Interactable.OnInteract`
  (params (Interactor :type "InteractorComponent Object Reference") (Interactable :type "InteractableComponent Object Reference"))
  (`/Engine/EditorBlueprintResources/StandardMacros.DoOnce` false
    (:`Completed`
      (goto _label))))

(event `BloquearPuerta`
  (set `self.estaBloqueada?` true)
  (`KismetSystemLibrary.PrintString` "cerrar puerta")
  (goto _label :!via `Reverse`))

(fn `UserConstructionScript`
  (`InteractableComponent.SetTooltipText` (`self.Interactable`) "Open"))