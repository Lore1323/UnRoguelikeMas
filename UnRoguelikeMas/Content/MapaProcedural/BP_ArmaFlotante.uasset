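; BP_ArmaFlotante is a weapon pickup that gives its weapon to the player on interaction.
; On BeginPlay it configures its Interactable component from the "Weapon" row of DT_CIP_InteractableList and sets its mesh from the DT_Weapons row keyed by IDArma.
; Sphere overlap caches the BP_PlayerEnzo reference, never cleared here.
; OnInteract passes IDArma to that player's RecibirArma, then destroys the pickup.
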(event `self.ReceiveBeginPlay`
  (`InteractableComponent.SetInteractableDataBasedOnDataTable` (`self.Interactable`) "/CustomizableInteractionPlugin/Blueprint/Interactables/DT_CIP_InteractableList.DT_CIP_InteractableList" "Weapon")
  (bind _returnvalue (`|GetDataTableRow` "/Game/Weapons/DT_Weapons.DT_Weapons" (`KismetStringLibrary.Conv_StringToName` (`KismetStringLibrary.Conv_IntToString` (`self.IDArma`))))
    (:`then`
      (set `SkeletalMeshComponent.SkeletalMeshAsset` (`.Mesh_20_5885BAE3419C281D3A4C5AA8671BE0AA` (break `/Game/Weapons/S_WeaponStats` _returnvalue)) (`self.WeaponMesh`)))))

(event `self.Sphere.OnComponentBeginOverlap`
  (params (OverlappedComponent :type "PrimitiveComponent Object Reference") (OtherActor :type "Actor Object Reference") (OtherComp :type "PrimitiveComponent Object Reference") (OtherBodyIndex :type Integer) (bFromSweep :type Boolean) (SweepResult :type "HitResult Structure (by ref)"))
  (bind _asbp_player_enzo_ (cast `/Game/PlayerEnzo/BP_PlayerEnzo+` OtherActor))
  (set `self.As BP Player Enzo+` _asbp_player_enzo_))

(event `self.Interactable.OnInteract`
  (params (Interactor :type "InteractorComponent Object Reference") (Interactable :type "InteractableComponent Object Reference"))
  (`/Game/PlayerEnzo/BP_PlayerEnzo+.RecibirArma` (`self.As BP Player Enzo+`) (`self.IDArma`))
  (`self.K2_DestroyActor`))

(fn `UserConstructionScript`)