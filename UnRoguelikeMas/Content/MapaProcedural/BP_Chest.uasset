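; Interactable loot chest that opens once and spawns a random floating weapon pickup.
; An Interactable component, configured from the Chest DataTable row, triggers a timeline that rotates the lid mesh open from its initial rotation.
; When that finishes, a second timeline spawns BP_ArmaFlotante once with a random LootPosible ID while nudging the spawn point upward, without attaching the weapon to it.
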(event `self.ReceiveBeginPlay`
  (`InteractableComponent.SetInteractableDataBasedOnDataTable` (`self.Interactable`) "/CustomizableInteractionPlugin/Blueprint/Interactables/DT_CIP_InteractableList.DT_CIP_InteractableList" "Chest")
  (set `self.rotInit` (`SceneComponent.K2_GetComponentRotation` (`self.SM_Chest`))))

(event `self.Interactable.OnOverlapUpdated`
  (params (bIsOverlapping :type Boolean) (OverlappingInteractor :type "InteractorComponent Object Reference") (Interactable :type "InteractableComponent Object Reference"))
  (bind _returnvalue (`GameplayStatics.GetActorOfClass` "/Game/PlayerEnzo/BP_PlayerEnzo+.BP_PlayerEnzo+_C"))
  (set `self.player` _returnvalue))

(event `self.Interactable.OnInteract`
  (params (Interactor :type "InteractorComponent Object Reference") (Interactable :type "InteractableComponent Object Reference"))
  (bind _rotinit (`self.rotInit`))
  ; Chest Opening Anim
  (`/Engine/EditorBlueprintResources/StandardMacros.DoOnce` false
    (:`Completed`
      (bind (_direction _alpha) (`Timeline|Open Chest`)
        (:`Update`
          (`SceneComponent.K2_SetWorldRotation` (`self.SM_Chest`) (`KismetMathLibrary.RLerp` _rotinit (`KismetMathLibrary.ComposeRotators` _rotinit (struct :`Roll` -150.0)) _alpha) true false))
        (:`Finished`
          (`self.Spawning weapon`))))))

(event `Spawning weapon`
  (bind _returnvalue (`SceneComponent.K2_GetComponentLocation` (`self.Spawnpoint Item`)))
  (bind (_direction _alpha) (`Timeline|Item`)
    (:`Update`
      (`|ExecutionSequence`
        (:`then_0`
          (`/Engine/EditorBlueprintResources/StandardMacros.DoOnce` false
            (:`Completed`
              (`|SpawnActorFromClass` "/Game/MapaProcedural/BP_ArmaFlotante.BP_ArmaFlotante_C" (`SceneComponent.K2_GetComponentToWorld` (`self.Spawnpoint Item`)) "AlwaysSpawn" "MultiplyWithRoot" null (`KismetArrayLibrary.Array_Random` (`self.lootPosible`)) null))))
        (:`then_1`
          (`SceneComponent.K2_SetWorldLocation` (`self.Spawnpoint Item`) (`KismetMathLibrary.VLerp` _returnvalue (+ _returnvalue (0.0 0.0 1.0)) _alpha) true false))))))

(fn `UserConstructionScript`)