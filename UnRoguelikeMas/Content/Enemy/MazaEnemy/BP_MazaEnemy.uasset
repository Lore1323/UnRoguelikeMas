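; BP_MazaEnemy is a melee enemy that chases BP_PlayerEnzo and attacks with a combo montage.
; BeginPlay sets health and damage, then starts an AI MoveTo loop that retries after failure, attacks on success, and resumes chasing when the montage completes.
; MeleeTrace hits apply damage only to the player.
; The construction script links the modular skeletal meshes to the main Mesh through leader pose.
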(event `self.ReceiveBeginPlay`
  ; Seteo de cosas
  (set `self.Vida` 75.0)
  (set `self.Damage` 25.0)
  (bind _returnvalue (`GameplayStatics.GetActorOfClass` "/Game/PlayerEnzo/BP_PlayerEnzo+.BP_PlayerEnzo+_C"))
  (set `self.Player` _returnvalue)
  (`self.Follow Player`))

(event `Follow Player`
  ; Seguir al Player
  (`|AIMoveTo` self (0.0 0.0 0.0) (`self.Player`)
    (:`OnSuccess`
      (`self.Attack Player`))
    (:`OnFail`
      (`KismetSystemLibrary.Delay` 0.5)
      (`self.Follow Player`))))

(event `Attack Player`
  ; atacar
  (`|PlayMontage` (`self.Mesh`) "/Game/Enemy/MazaEnemy/Anim/standing_melee_combo_attack_ver__1_Montage.standing_melee_combo_attack_ver__1_Montage" 1.0 0.0 "None" false
    (:`OnCompleted`
      (`self.Follow Player`))))

(event `self.MeleeTrace.OnTraceHit`
  (params (ThisComponent :type "MeleeTraceComponent Object Reference") (HitActor :type "Actor Object Reference") (HitLocation :type "Vector Structure (by ref)") (HitNormal :type "Vector Structure (by ref)") (HitBoneName :type Name) (TraceHandle :type "MeleeTraceInstanceHandle Structure"))
  ; Aplicar Daño
  (bind _asbp_player_enzo_ (cast `/Game/PlayerEnzo/BP_PlayerEnzo+` HitActor))
  (`GameplayStatics.ApplyDamage` _asbp_player_enzo_ (`self.Damage`)))

(fn `UserConstructionScript`
  (`SkinnedMeshComponent.SetLeaderPoseComponent` (`self.SkeletalMesh2`) (`self.Mesh`) false false)
  (`SkinnedMeshComponent.SetLeaderPoseComponent` (`self.SkeletalMesh3`) (`self.Mesh`) false false)
  (`SkinnedMeshComponent.SetLeaderPoseComponent` (`self.SkeletalMesh4`) (`self.Mesh`) false false)
  (`SkinnedMeshComponent.SetLeaderPoseComponent` (`self.SkeletalMesh5`) (`self.Mesh`) false false)
  (`SkinnedMeshComponent.SetLeaderPoseComponent` (`self.SkeletalMesh6`) (`self.Mesh`) false false)
  (`SkinnedMeshComponent.SetLeaderPoseComponent` (`self.SkeletalMesh`) (`self.Mesh`) false false)
  (`SkinnedMeshComponent.SetLeaderPoseComponent` (`self.SkeletalMesh1`) (`self.Mesh`) false false))