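; Ranged enemy that cycles between repositioning, aiming at BP_PlayerEnzo and firing a crossbow.
; It moves to random reachable navmesh points, then a timeline turns it toward the player while a line trace checks visibility.
; A visible player triggers the shoot montage, otherwise it relocates; the separate Shoot event spawns BP_Arrow, plays reload and restarts the cycle.
; The construction script links modular meshes to the main mesh's pose.
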(event `Reposicionamiento`
  ; Reposicionarse
  (`TimelineComponent.Stop` (`self.TiempoDeApuntado`))
  (`|AIMoveTo` self (`NavigationSystemV1.K2_GetRandomReachablePointInRadius` (`SceneComponent.K2_GetComponentLocation` (`self.Mesh`)) 2000.0 null "/Script/AIModule.NavFilter_AIControllerDefault") null
    (:`OnSuccess`
      _)
    (:`OnFail`
      _))
  (`self.MirarAlPlayer`))

(event `Shoot`
  (bind (_returnvalue_roll _returnvalue_pitch _returnvalue_yaw) (`KismetMathLibrary.BreakRotator` (`self.K2_GetActorRotation`)))
  (bind _arrow1 (`self.Arrow1`))
  (bind (_returnvalue_location _returnvalue_rotation) (`KismetMathLibrary.BreakTransform` (`SceneComponent.K2_GetComponentToWorld` _arrow1)))
  ; Disparo y Anim de recarga
  (`SceneComponent.K2_SetWorldRotation` _arrow1 (`KismetMathLibrary.MakeRotator` _returnvalue_roll (+ _returnvalue_pitch 1.0) _returnvalue_yaw) false true)
  (`|SpawnActorFromClass` "/Game/SKnight_modular/Skeleton_Knight_07/mesh/weapon/BP_Arrow.BP_Arrow_C" (`KismetMathLibrary.MakeTransform` _returnvalue_location _returnvalue_rotation (2.0 2.0 2.0)) "AlwaysSpawn" "MultiplyWithRoot" null null)
  (`|PlayMontage` (`self.Weapon`) "/Game/SKnight_modular/Skeleton_Knight_07/mesh/weapon/AM_Reload.AM_Reload" 0.5
    (:`then`
      (`TimelineComponent.Stop` (`self.TiempoDeApuntado`)))
    (:`OnCompleted`
      (`KismetSystemLibrary.Delay` 0.2)
      (`self.Reposicionamiento `))))

(event `PlayMontage`
  ; Reproducir montage
  (`|PlayMontage` (`self.Weapon`) "/Game/SKnight_modular/Skeleton_Knight_07/mesh/weapon/AM_Shoot.AM_Shoot" 1.0 0.0 "None" false))

(event `self.ReceiveBeginPlay`
  ; Seteo de estadisticas
  (set `self.Vida` 60.0)
  (set `self.Montages` (`|MakeArray` null null null null null :!type "AnimMontage Object Reference"))
  (bind _returnvalue (`GameplayStatics.GetActorOfClass` "/Game/PlayerEnzo/BP_PlayerEnzo+.BP_PlayerEnzo+_C"))
  (set `self.Player` _returnvalue)
  (`self.Reposicionamiento `))

(event `MirarAlPlayer`
  ; Girar Siguiendo Al Player
  (`|ExecutionSequence`
    (:`then_0`
      (bind (_direction _newtrack_0) (`Timeline|TiempoDeApuntado`)
        (:`Update`
          (`self.SetRotationToPlayer` _newtrack_0)
          (`self.ChequearPlayer`))))
    (:`then_1`
      (`KismetSystemLibrary.Delay` 1.0)
      (if (`self.playerVisto`)
        (`KismetSystemLibrary.Delay` 1.0)
        (`self.PlayMontage`)
        (else
          (`self.Reposicionamiento `))))))

(fn `ChequearPlayer`
  (bind _outhit (`KismetSystemLibrary.LineTraceSingle` :`Start` (`SceneComponent.K2_GetComponentLocation` (`self.Weapon`)) :`End` (`SceneComponent.K2_GetComponentLocation` (`Character.CapsuleComponent` (`self.Player`))) :`TraceChannel` "TraceTypeQuery1" :`DrawDebugType` "ForOneFrame"))
  (if (== (`.HitActor` (`GameplayStatics.BreakHitResult` _outhit)) (`self.Player`))
    (set `self.playerVisto` true)
    (else
      (set `self.playerVisto` false))))

(fn `GetSocketLocation`
  (set `self.socketCrossbow` (`SceneComponent.GetSocketLocation` (`self.Weapon`) "weaponSocket")))

(fn `SetRotationToPlayer`
  (params (DeltaTime :type "Float (single-precision)"))
  (`self.K2_SetActorRotation` (`KismetMathLibrary.RInterpTo` (`self.K2_GetActorRotation`) (`KismetMathLibrary.FindLookAtRotation` (`SceneComponent.K2_GetComponentLocation` (`self.Mesh`)) (`SceneComponent.K2_GetComponentLocation` (`Character.Mesh` (`self.Player`)))) DeltaTime 0.0)))

(fn `UserConstructionScript`
  (`SkinnedMeshComponent.SetLeaderPoseComponent` (`self.SkeletalMesh7`) (`self.Mesh`) false false)
  (`SkinnedMeshComponent.SetLeaderPoseComponent` (`self.SkeletalMesh2`) (`self.Mesh`) false false)
  (`SkinnedMeshComponent.SetLeaderPoseComponent` (`self.SkeletalMesh3`) (`self.Mesh`) false false)
  (`SkinnedMeshComponent.SetLeaderPoseComponent` (`self.SkeletalMesh4`) (`self.Mesh`) false false)
  (`SkinnedMeshComponent.SetLeaderPoseComponent` (`self.SkeletalMesh5`) (`self.Mesh`) false false)
  (`SkinnedMeshComponent.SetLeaderPoseComponent` (`self.SkeletalMesh6`) (`self.Mesh`) false false)
  (`SkinnedMeshComponent.SetLeaderPoseComponent` (`self.SkeletalMesh7`) (`self.Mesh`) false false)
  (`SkinnedMeshComponent.SetLeaderPoseComponent` (`self.SkeletalMesh`) (`self.Mesh`) false false)
  (`SkinnedMeshComponent.SetLeaderPoseComponent` (`self.SkeletalMesh1`) (`self.Mesh`) false false)
  (`SkinnedMeshComponent.SetLeaderPoseComponent` (`self.SkeletalMesh8`) (`self.Mesh`) false false)
  (`SkinnedMeshComponent.SetLeaderPoseComponent` (`self.SkeletalMesh9`) (`self.Mesh`) false false))