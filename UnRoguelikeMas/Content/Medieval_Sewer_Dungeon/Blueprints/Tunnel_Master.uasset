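; Master tunnel piece for the sewer dungeon that, when flagged as a room, becomes a locked-door combat encounter.
; It spawns a door at its start point, then locks it and spawns enemies when the player first enters the trigger.
; A random wave from the difficulty-curve DataTable row, keyed by GameInstance difficulty, fills random spawnpoints with enemies told of the player.
; Death events empty the enemy list, unlocking the door and notifying the GameInstance.
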(event `self.ReceiveBeginPlay`
  (if (`self.isARoom`)
    (bind _returnvalue (`|SpawnActorFromClass` "/Game/MapaProcedural/BP_Doors.BP_Doors_C" (`SceneComponent.K2_GetComponentToWorld` (`self.StartPoint`)) "AlwaysSpawn" "MultiplyWithRoot" null "0.000000,0.000000,-800.000000|0.000000,0.000000,0.000000|1.000000,1.000000,1.000000" null))
    (set `self.puertaDeEntrada` _returnvalue)))

(event `Make List spawnpoint`
  (`KismetArrayLibrary.Array_Append` (`self.spawnpointList`) (`SceneComponent.GetChildrenComponents` (`self.Spawnpoints`) true)))

(event `self.StartSpawner.OnComponentBeginOverlap`
  (params (OverlappedComponent :type "PrimitiveComponent Object Reference") (OtherActor :type "Actor Object Reference") (OtherComp :type "PrimitiveComponent Object Reference") (OtherBodyIndex :type Integer) (bFromSweep :type Boolean) (SweepResult :type "HitResult Structure (by ref)"))
  (bind _puertadeentrada (`self.puertaDeEntrada`))
  (`/Engine/EditorBlueprintResources/StandardMacros.DoOnce` false
    (:`Completed`
      (bind _asbp_player_enzo_ (cast `/Game/PlayerEnzo/BP_PlayerEnzo+` OtherActor))
      (if (`self.isARoom`)
        (`/Engine/EditorBlueprintResources/StandardMacros.IsValid` _puertadeentrada
          (:`Is Valid`
            (`/Game/MapaProcedural/BP_Doors.BloquearPuerta` _puertadeentrada)
            (`self.Spawnear` _asbp_player_enzo_)))))))

(event `Spawnear`
  (params (player :type "/Game/PlayerEnzo/BP_PlayerEnzo+ Object Reference"))
  (bind (_returnvalue_location _returnvalue_rotation _returnvalue_scale) (`KismetMathLibrary.BreakTransform` (`SceneComponent.K2_GetComponentToWorld` (`KismetArrayLibrary.Array_Random` (`self.spawnpointList`)))))
  ; Spawnear Enemigos
  (bind _dificultad (message `/Game/MapaProcedural/BPI_GestorDeDificultad.ObtenerDificultadActual` (`GameplayStatics.GetGameInstance`)))
  (bind _returnvalue (`|GetDataTableRow` "/Game/SistemaDeOleadas/DT_CurvaDeDificultad.DT_CurvaDeDificultad" (`KismetStringLibrary.Conv_StringToName` (`KismetStringLibrary.Conv_IntToString` _dificultad)))
    (:`then`
      (for _array_element (`.grupoDeEnemigos_3_6311A1F74D5EDE650873AE815B61A3CF` (break `/Game/SistemaDeOleadas/S_DefinicionDeOleadas` (`KismetArrayLibrary.Array_Random` (`.DefinicionDeOleadas_3_F905C66741CB02FF1812A78FD385ACBD` (break `/Game/SistemaDeOleadas/S_FilaDeDificultad` _returnvalue)))))
        (for _ (range (+ (`.cantidadDeEnemigos_4_FDCB83714806C1CAE661E58F5E192EEE` (break `/Game/SistemaDeOleadas/S_GrupoDeEnemigos` _array_element)) 1))
          (bind _returnvalue_2 (`|SpawnActorFromClass` (break `/Game/SistemaDeOleadas/S_GrupoDeEnemigos` _array_element) (`KismetMathLibrary.MakeTransform` (+ _returnvalue_location (0.0 0.0 10.0)) (struct) _returnvalue_scale) "AlwaysSpawn" "OverrideRootScale" null 100.0 null))
          (message `/Game/PlayerEnzo/BPI_PlayerChase.AvisarDondeEstaElPlayer` _returnvalue_2 player)
          (`KismetArrayLibrary.Array_Add` (`self.cantidadDeEnemigos`) _returnvalue_2)
          (add `/Game/Enemy/BP_DadEnemy.Mori` _returnvalue_2 (delegate `A Muerto un enemigo`)))))))

(event `A Muerto un enemigo`
  (params (EnemigoMuerto :type "/Game/Enemy/BP_DadEnemy Object Reference"))
  (bind _cantidaddeenemigos (`self.cantidadDeEnemigos`))
  ; Spawnear Enemigos
  (`KismetArrayLibrary.Array_RemoveItem` _cantidaddeenemigos EnemigoMuerto)
  (if (== (`KismetArrayLibrary.Array_Length` _cantidaddeenemigos) 0)
    (`/Game/MapaProcedural/BP_Doors.DesbloquearPuerta` (`self.puertaDeEntrada`))
    (message `/Game/MapaProcedural/BPI_GestorDeDificultad.AvisarSalaDespejada` (`GameplayStatics.GetGameInstance`))))

(fn `UserConstructionScript`)